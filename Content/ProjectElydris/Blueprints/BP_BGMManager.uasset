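; BP_BGMManager is a background music manager that sets BGM volume from the options model.
; UpdateFromModel multiplies master and music volume into the BGMAudio volume multiplier and prints debug text, called by an audio-changed handler or CallUpdateModel.
; BeginPlay only casts the GameInstance to GameManager; fetching the options model and the looping refresh timer are disconnected and never run.
; No binding for the audio-changed handler appears in the graph.
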(event `CallUpdateModel`
  (`self.UpdateFromModel`))

(event `UpdateFromModel`
  (bind _optionsmodelref (`self.OptionsModelRef`))
  (`KismetSystemLibrary.PrintString` "\"BGM: Master=\" + MasterVolume + \" Music=\" + MusicVolume")
  (`AudioComponent.SetVolumeMultiplier` (`self.BGM_Audio`) (* (`OptionsModel.MasterVolume` _optionsmodelref) (`OptionsModel.MusicVolume` _optionsmodelref))))

(event `self.ReceiveBeginPlay`
  (bind _asgame_manager (cast `GameManager` (`GameplayStatics.GetGameInstance`))))

(event `OnAudioChanged_Handler`
  (`KismetSystemLibrary.PrintString` "\"BGM: OnAudioChanged\"")
  (`self.UpdateFromModel`))

(fn `UserConstructionScript`)